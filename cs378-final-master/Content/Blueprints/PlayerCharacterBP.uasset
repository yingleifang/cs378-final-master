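; Player character Blueprint that handles movement, sprinting, jumping and projectile shooting.
; Move, jump and landing events check CanPerformAction against an action state; moves and jumps then update that state.
; Sprint scales max walk speed by SprintMod and divides it back on end.
; Shoot clears CanShoot, plays a sound and spawns a ProjectileBP at the capsule, aimed along the spring arm, passing on its IsDestroy flag.
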(event EventShoot
  (params (isDestroy :type Boolean))
  (if (Variables|Default|GetCanShoot)
    (Variables|Default|SetCanShoot false)
    (Audio|PlaySoundatLocation "/Game/Sounds/swordSwing.swordSwing" (Transformation|GetActorLocation) "0, 0, 0" 1.0 1.0 0.0 0 0 0) ; Play firing sound
    (bind _returnvalue (Game|SpawnActorfromClass "/Game/Blueprints/ProjectileBP.ProjectileBP_C" (Math|Transform|MakeTransform (Transformation|GetWorldLocation (Variables|Default|GetCapsuleComponent)) (Transformation|GetWorldRotation (Variables|Default|GetSpringArm))) "AdjustIfPossibleButAlwaysSpawn" 0 0))
    (Variables|/Game/Blueprints/ProjectileBP.ProjectileBP_C|SetIsDestroy _returnvalue isDestroy)))

(event EventMoveForward
  (params (value :type Float%20%28single-precision%29))
  (switch Utilities|FlowControl|Switch|SwitchonECharacterActionStateEnum (Variables|Default|GetCharacterActionState)
    (:IDLE
      _)
    (:MOVE
      _)
    (:JUMP
      _))
  (bind _returnvalue (Class|PlayerCharacter|CanPerformAction "MOVE"))
  (if _returnvalue
    (Class|PlayerCharacter|DoMoveForward value)
    (Class|PlayerCharacter|UpdateActionState "MOVE")))

(event EventStartSprint
  (bind _charactermovement (Variables|Character|GetCharacterMovement))
  (Variables|/Script/Engine.CharacterMovementComponent|SetMaxWalkSpeed _charactermovement (* (Variables|/Script/Engine.CharacterMovementComponent|GetMaxWalkSpeed _charactermovement) (Variables|Default|GetSprintMod))))

(event EventEndSprint
  (bind _charactermovement (Variables|Character|GetCharacterMovement))
  (Variables|/Script/Engine.CharacterMovementComponent|SetMaxWalkSpeed _charactermovement (/ (Variables|/Script/Engine.CharacterMovementComponent|GetMaxWalkSpeed _charactermovement) (Variables|Default|GetSprintMod))))

(event EventJumpInit
  (bind _returnvalue (Class|PlayerCharacter|CanPerformAction "JUMP"))
  (if _returnvalue
    (Character|Jump)
    (Class|PlayerCharacter|JumpAction)
    (Class|PlayerCharacter|UpdateActionState "JUMP")
    (else
      (Development|PrintString "Cannot Jump"))))

(event EventMoveRight
  (params (value :type Float%20%28single-precision%29))
  (switch Utilities|FlowControl|Switch|SwitchonECharacterActionStateEnum (Variables|Default|GetCharacterActionState)
    (:IDLE
      _)
    (:MOVE
      _)
    (:JUMP
      _))
  (bind _returnvalue (Class|PlayerCharacter|CanPerformAction "MOVE"))
  (if _returnvalue
    (Class|PlayerCharacter|DoMoveRight value)
    (Class|PlayerCharacter|UpdateActionState "MOVE")))

(event EventOnLanded
  (params (Hit :type Hit%20Result%20Structure%20%28by%20ref%29))
  (bind _returnvalue (Class|PlayerCharacter|CanPerformAction "IDLE"))
  (if _returnvalue
    (Class|PlayerCharacter|FinalizeJump)))

(fn ConstructionScript)