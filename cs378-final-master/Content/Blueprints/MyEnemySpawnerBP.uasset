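; Enemy spawner that periodically spawns a set number of Jumper actors around the player.
; A delayed-loop macro calls SpawnCharacter, which line-traces downward from high above random points in the MaxDistance component's bounds and spawns at the hit with a random yaw.
; Each Tick, it eases toward a point behind the player and drags the NavMeshBoundsVolume along with it.
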(event EventBeginPlay
  (Utilities|ForLoopwithDelay 1 (Variables|Default|GetSpawnAmount) 5.0
    (:Loop%20Body
      (CallFunction|SpawnCharacter))))

(event EventTick
  (params (DeltaSeconds :type Float%20%28single-precision%29))
  (bind _returnvalue (Game|Player|GetPlayerPawn 0))
  (bind _returnvalue_2 (Transformation|GetActorLocation))
  (bind _returnvalue_3 (Transformation|GetActorLocation _returnvalue))
  (bind _returnvalue_4 (Transformation|GetActorForwardVector _returnvalue))
  (bind _returnvalue_5 (* _returnvalue_4 -150))
  (bind _returnvalue_6 (+ _returnvalue_3 _returnvalue_5))
  (bind _returnvalue_7 (Math|Interpolation|VInterpTo _returnvalue_2 _returnvalue_6 DeltaSeconds 3.0))
  (Utilities|FlowControl|Sequence
    (:then_0
      (bind _returnvalue_8 (Actor|GetActorOfClass "/Script/NavigationSystem.NavMeshBoundsVolume"))
      (Transformation|SetActorLocation _returnvalue_8 _returnvalue_7 false true))
    (:then_1
      (Transformation|SetActorLocation _returnvalue_7 false true))))

(fn ConstructionScript)

(fn SpawnCharacter
  (bind _maxdistance (Variables|Default|GetMaxDistance))
  (bind (_origin _boxextent) (Collision|GetComponentBounds _maxdistance))
  (bind _returnvalue (Math|Random|RandomPointinBoundingBox _origin _boxextent))
  (bind (_x _y _z) (Math|Vector|BreakVector _returnvalue))
  (bind _returnvalue_2 (+ _z 5e+04))
  (bind _returnvalue_3 (Math|Vector|MakeVector _x _y _returnvalue_2))
  (bind _outhit (Collision|LineTraceForObjects _returnvalue_3 (+ (* (* (Transformation|GetActorUpVector) -1) 5.5e+04) _returnvalue_3) (Utilities|Array|MakeArray "ObjectTypeQuery1") false 0 "ForDuration"))
  (Game|SpawnActorfromClass "/Game/Blueprints/Jumper.Jumper_C" (Math|Transform|MakeTransform (.ImpactPoint (Collision|BreakHitResult _outhit)) (Math|Rotator|MakeRotator 0.0 0.0 (Math|Random|RandomFloat))) "AdjustIfPossibleButDontSpawnIfColliding" 0 0))