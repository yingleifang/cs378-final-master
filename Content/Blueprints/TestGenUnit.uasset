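; TestGenUnit is a procedural terrain patch actor, built in the construction script from simplex noise.
; Nested loops create a grid of quads sized by UnitSize, each its own ProceduralMesh section with collision and a concrete grime material.
; Corner heights sample noise at world XY using InFactor, scaled by HeightMultiplier, so shared edges match and the shape depends on actor location.
; The event graph is empty.
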(event EventBeginPlay)

(event Collision|EventActorBeginOverlap
  (params (OtherActor :type Actor%20Object%20Reference)))

(event EventTick
  (params (DeltaSeconds :type Float%20%28single-precision%29)))

(fn ConstructionScript
  (bind _length (Variables|Default|GetLength))
  (bind _unitsize (Variables|Default|GetUnitSize))
  (bind _infactor (Variables|Default|GetInFactor))
  (bind _unitsize_2 (Variables|Default|GetUnitSize))
  (bind _proceduralmesh (Variables|Default|GetProceduralMesh))
  (bind _defaultsceneroot (Variables|Default|GetDefaultSceneRoot))
  (bind _returnvalue (Transformation|GetWorldLocation _defaultsceneroot))
  (bind _returnvalue_2 (Math|Conversions|ToFloat(Integer) _unitsize))
  (bind (_x _y) (Math|Vector|BreakVector _returnvalue))
  (for _index (range 0 (Variables|Default|GetLength))
    (for _index_2 (range 0 _length)
      (bind _returnvalue_3 (Class|SimplexNoiseBPLibrary|GetSimplexNoise2DEX (+ _x (Math|Conversions|ToFloat(Integer) (* _index _unitsize_2))) (+ _y (Math|Conversions|ToFloat(Integer) (* _index_2 _unitsize_2))) 2.3 0.6 4 _infactor false))
      (bind _returnvalue_4 (Class|SimplexNoiseBPLibrary|GetSimplexNoise2DEX (+ _x (Math|Conversions|ToFloat(Integer) (* _index _unitsize_2))) (+ (+ _y (Math|Conversions|ToFloat(Integer) (* _index_2 _unitsize_2))) _returnvalue_2) 2.3 0.6 4 _infactor false))
      (bind _returnvalue_5 (Class|SimplexNoiseBPLibrary|GetSimplexNoise2DEX (+ (Math|Conversions|ToFloat(Integer) (Variables|Default|GetUnitSize)) (+ _x (Math|Conversions|ToFloat(Integer) (* _index _unitsize_2)))) (+ _y (Math|Conversions|ToFloat(Integer) (* _index_2 _unitsize_2))) 2.3 0.6 4 _infactor false))
      (bind _returnvalue_6 (Class|SimplexNoiseBPLibrary|GetSimplexNoise2DEX (+ (Math|Conversions|ToFloat(Integer) (Variables|Default|GetUnitSize)) (+ _x (Math|Conversions|ToFloat(Integer) (* _index _unitsize_2)))) (+ (+ _y (Math|Conversions|ToFloat(Integer) (* _index_2 _unitsize_2))) (Math|Conversions|ToFloat(Integer) (Variables|Default|GetUnitSize))) 2.3 0.6 4 _infactor false))
      (Class|ProceduralMeshComponent|CreateMeshSectionLinearColor _proceduralmesh (+ (* _index _length) _index_2) (Utilities|Array|MakeArray (Math|Vector|MakeVector (Math|Conversions|ToFloat(Integer) (* _index _unitsize_2)) (Math|Conversions|ToFloat(Integer) (* _index_2 _unitsize_2)) (* _returnvalue_3 (Variables|Default|GetHeightMultiplier))) (Math|Vector|MakeVector (Math|Conversions|ToFloat(Integer) (* _index _unitsize_2)) (+ (Math|Conversions|ToFloat(Integer) (* _index_2 _unitsize_2)) _returnvalue_2) (* _returnvalue_4 (Variables|Default|GetHeightMultiplier))) (Math|Vector|MakeVector (+ _returnvalue_2 (Math|Conversions|ToFloat(Integer) (* _index _unitsize_2))) (Math|Conversions|ToFloat(Integer) (* _index_2 _unitsize_2)) (* _returnvalue_5 (Variables|Default|GetHeightMultiplier))) (Math|Vector|MakeVector (+ _returnvalue_2 (Math|Conversions|ToFloat(Integer) (* _index _unitsize_2))) (+ (Math|Conversions|ToFloat(Integer) (* _index_2 _unitsize_2)) _returnvalue_2) (* _returnvalue_6 (Variables|Default|GetHeightMultiplier)))) (Utilities|Array|MakeArray 0 1 2 3 2 1) 0 (Utilities|Array|MakeArray "(X=0.000000,Y=0.000000)" "(X=0.000000,Y=1.000000)" "(X=1.000000,Y=0.000000)" "(X=1.000000,Y=1.000000)") 0 0 0 0 0 true)
      (Rendering|Material|SetMaterial _proceduralmesh (+ (* _index _length) _index_2) "/Game/StarterContent/Materials/M_Concrete_Grime.M_Concrete_Grime"))))