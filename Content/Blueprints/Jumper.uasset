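; Jumper is an actor that jumps periodically and is destroyed by projectiles.
; Tick accumulates delta time and calls Jump each time it passes TimeTillJump, then resets the timer.
; Overlapping a ProjectileBP or any subclass plays the Hit sound at the actor's location and destroys the Jumper.
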(event Collision|EventActorBeginOverlap
  (params (OtherActor :type Actor%20Object%20Reference))
  (if (Utilities|ClassIsChildOf (Utilities|GetClass OtherActor) "/Game/Blueprints/ProjectileBP.ProjectileBP_C")
    (Audio|PlaySoundatLocation "/Game/Sounds/hit.hit" (Transformation|GetActorLocation) "0, 0, 0" 1.0 1.0 0.0 0 0 0)
    (Actor|DestroyActor)))

(event EventTick
  (params (DeltaSeconds :type Float%20%28single-precision%29))
  (bind _output_get (Variables|Default|SetCurTime (+ DeltaSeconds (Variables|Default|GetCurTime))))
  (if (> _output_get (Variables|Default|GetTimeTillJump))
    (Variables|Default|SetCurTime 0.0)
    (Character|Jump)))

(fn ConstructionScript)